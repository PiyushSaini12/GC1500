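; Checkpoint and lap tracker for a racing game, using one trigger box that hops through eight checkpoint meshes in order.
; Ending an overlap moves the box to the next checkpoint's transform, with a resettable DoOnce debouncing the advance, while beginning an overlap plays a sound.
; After the eighth checkpoint it increments the lap and, within the lap limit, returns to the first and has MainHUD check the record and reset lap time.
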(event OnComponentEndOverlap(CP_TriggerBox_CollisionComp)
  (params (OverlappedComponent :type Primitive%20Component%20Object%20Reference) (OtherActor :type Actor%20Object%20Reference) (OtherComp :type Primitive%20Component%20Object%20Reference) (OtherBodyIndex :type Integer))
  (bind _cp_1_staticmeshcomponent0 (Variables|Default|GetCP_1_StaticMeshComponent0))
  (bind _returnvalue (Transformation|GetWorldTransform _cp_1_staticmeshcomponent0))
  (bind (_location _rotation) (Math|Transform|BreakTransform _returnvalue))
  (if (== (Variables|Default|GetCP_Count) 8)
    (Utilities|FlowControl|Delay 0.2)
    (Variables|Default|SetCP_Count 1)
    (Variables|Default|SetLAP (+ (Variables|Default|GetLAP) 1))
    (if (<= (Variables|Default|GetLAP) (Variables|Default|GetMAXLAP))
      (Transformation|SetWorldTransform (Variables|Default|GetCP_TriggerBox_CollisionComp) (Math|Transform|MakeTransform _location _rotation "14.000000,1,6.000000") false false)
      (bind _asmain_hud (Utilities|Casting|CastToMainHUD (HUD|GetHUD (Game|GetPlayerController 0))))
      (Variables|/Game/HUD/MainHUD.MainHUD_C|SetHUD_Lap _asmain_hud (Variables|Default|GetLAP))
      (Default|LapRecordCheck _asmain_hud)
      (Utilities|FlowControl|Delay 0.2)
      (Default|ResetLapTime _asmain_hud))
    (else
      (Utilities|FlowControl|DoOnce false :!label _label
        (:Completed
          (Transformation|SetWorldTransform (Variables|Default|GetCP_TriggerBox_CollisionComp) (Math|Transform|MakeTransform (.Location (Math|Transform|BreakTransform (Transformation|GetWorldTransform (Utilities|Array|Get(acopy) (Utilities|Array|MakeArray (Variables|Default|GetCP_1_StaticMeshComponent0) (Variables|Default|GetCP_2_StaticMeshComponent0) (Variables|Default|GetCP_3_StaticMeshComponent0) (Variables|Default|GetCP_4_StaticMeshComponent0) (Variables|Default|GetCP_5_StaticMeshComponent0) (Variables|Default|GetCP_6_StaticMeshComponent0) (Variables|Default|GetCP_7_StaticMeshComponent0) (Variables|Default|GetCP_8_StaticMeshComponent0)) (Variables|Default|GetCP_Count))))) (.Rotation (Math|Transform|BreakTransform (Transformation|GetWorldTransform (Utilities|Array|Get(acopy) (Utilities|Array|MakeArray (Variables|Default|GetCP_1_StaticMeshComponent0) (Variables|Default|GetCP_2_StaticMeshComponent0) (Variables|Default|GetCP_3_StaticMeshComponent0) (Variables|Default|GetCP_4_StaticMeshComponent0) (Variables|Default|GetCP_5_StaticMeshComponent0) (Variables|Default|GetCP_6_StaticMeshComponent0) (Variables|Default|GetCP_7_StaticMeshComponent0) (Variables|Default|GetCP_8_StaticMeshComponent0)) (Variables|Default|GetCP_Count))))) "14.000000,1,6.000000") false false)
          (Variables|Default|SetCP_Count (+ (Variables|Default|GetCP_Count) 1))
          (Utilities|FlowControl|Delay 1.0)
          (goto _label Reset))))))

(event OnComponentBeginOverlap(CP_TriggerBox_CollisionComp)
  (params (OverlappedComponent :type Primitive%20Component%20Object%20Reference) (OtherActor :type Actor%20Object%20Reference) (OtherComp :type Primitive%20Component%20Object%20Reference) (OtherBodyIndex :type Integer) (bFromSweep :type Boolean) (SweepResult :type Hit%20Result%20Structure%20%28by%20ref%29))
  (Audio|PlaySoundatLocation "/Game/GameAudio/Checkpoint_Sound.Checkpoint_Sound" "0, 0, 0" "0, 0, 0" 1.0 1.0 0.0 0 0 0))

(event EventBeginPlay
  (bind _asmain_hud (Utilities|Casting|CastToMainHUD (HUD|GetHUD (Game|GetPlayerController 0))))
  (Variables|/Game/HUD/MainHUD.MainHUD_C|SetHUD_Lap _asmain_hud (Variables|Default|GetLAP))
  (Variables|/Game/HUD/MainHUD.MainHUD_C|SetHUD_MaxLaps _asmain_hud (Variables|Default|GetMAXLAP)))

(fn ConstructionScript)